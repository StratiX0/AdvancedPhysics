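; BP_Hovercraft is a player-driven hovercraft that handles thrust, steering, boost and flip recovery through Enhanced Input.
; Thrust and steering set target speeds on BPMovementComponent, with boost multiplying thrust.
; Steering inverts at full reverse thrust.
; Flip works only when the vehicle's up vector is level or downward, applying an impulse away from its roof, then a delayed roll impulse to right it.
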(event Input|EnhancedActionEvents|EnhancedInputActionIA_Thrust
  (params (ActionValue :type Float%20%28double-precision%29) (ElapsedSeconds :type Float%20%28double-precision%29) (TriggeredSeconds :type Float%20%28double-precision%29) (InputAction :type Input%20Action%20Object%20Reference :default "/Game/03-Inputs/Actions/IA_Thrust.IA_Thrust"))
  (bind _bp_movementcomponent (Variables|Default|GetBP_MovementComponent))
  ;[0.2917 0 0] Thrust
  (:Triggered
    (Variables|/Game/01-Blueprints/Hover/Components/BP_MovementComponent.BP_MovementComponent_C|SetTargetSpeed _bp_movementcomponent (* ActionValue 1e+04 (Variables|Default|GetBoostMultiplier))))
  (:Completed
    (Variables|/Game/01-Blueprints/Hover/Components/BP_MovementComponent.BP_MovementComponent_C|SetTargetSpeed _bp_movementcomponent 0.0)))

(event Input|EnhancedActionEvents|EnhancedInputActionIA_Steer
  (params (ActionValue :type Float%20%28double-precision%29) (ElapsedSeconds :type Float%20%28double-precision%29) (TriggeredSeconds :type Float%20%28double-precision%29) (InputAction :type Input%20Action%20Object%20Reference :default "/Game/03-Inputs/Actions/IA_Steer.IA_Steer"))
  (bind _returnvalue (Input|EnhancedActionValues|GetIA_Thrust))
  (bind _bp_movementcomponent (Variables|Default|GetBP_MovementComponent))
  ;[0.2604 0 0] Steering
  (:Triggered
    (Variables|/Game/01-Blueprints/Hover/Components/BP_MovementComponent.BP_MovementComponent_C|SetTargetAngularSpeed _bp_movementcomponent (* ActionValue 3e+03 (Math|Float|SelectFloat (Math|Float|Sign(Float) _returnvalue) 1.0 (== _returnvalue -1.0)))))
  (:Completed
    (Variables|/Game/01-Blueprints/Hover/Components/BP_MovementComponent.BP_MovementComponent_C|SetTargetAngularSpeed _bp_movementcomponent 0.0)))

(event Input|EnhancedActionEvents|EnhancedInputActionIA_Flip
  (params (ActionValue :type Boolean) (ElapsedSeconds :type Float%20%28double-precision%29) (TriggeredSeconds :type Float%20%28double-precision%29) (InputAction :type Input%20Action%20Object%20Reference :default "/Game/03-Inputs/Actions/IA_Flip.IA_Flip"))
  (bind _vehicle (Variables|Default|GetVehicle))
  (bind _vehicle_2 (Variables|Default|GetVehicle))
  (bind _returnvalue (Math|Vector|GetUpVector _vehicle_2))
  ;[0.3281 0.02841 0] Flip
  (:Started
    (if (<= (Math|Vector|DotProduct (Math|Vector|MakeVector 0.0 0.0 1.0) _returnvalue) 0.0)
      (Physics|AddImpulse (Variables|Default|GetVehicle) (* _returnvalue -2e+06) "None" false)
      (Utilities|FlowControl|Delay 0.1)
      (Class|PrimitiveComponent|AddAngularImpulseinDegrees _vehicle (* (Math|Vector|GetForwardVector _vehicle) 1e+09) "None" false))))

(event Input|EnhancedActionEvents|EnhancedInputActionIA_Boost
  (params (ActionValue :type Boolean) (ElapsedSeconds :type Float%20%28double-precision%29) (TriggeredSeconds :type Float%20%28double-precision%29) (InputAction :type Input%20Action%20Object%20Reference :default "/Game/03-Inputs/Actions/IA_Boost.IA_Boost"))
  ;[0.3698 0 0] Flip
  (:Started
    (Variables|Default|SetBoostMultiplier 3.0))
  (:Completed
    (Variables|Default|SetBoostMultiplier 1.0)))

(event EventBeginPlay
  (bind _returnvalue (Game|GetPlayerController 0))
  (bind _returnvalue_2 (PlayerController|LocalPlayerSubsystems|GetEnhancedInputLocalPlayerSubsystem _returnvalue))
  (Utilities|IsValid _returnvalue_2
    (:Is%20Valid
      (Input|AddMappingContext _returnvalue_2 "/Game/03-Inputs/IMC_Hovercraft.IMC_Hovercraft" 0 "(bIgnoreAllPressedKeysUntilRelease=True,bForceImmediately=False,bNotifyUserSettings=False)"))))

(fn ConstructionScript)