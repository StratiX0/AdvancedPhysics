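; Health component that tracks an actor's health and destroys the owner when it runs out.
; Health starts at MaxHealth on BeginPlay.
; ReceiveDamage subtracts damage and prints the remaining value, or clamps Health to zero and calls Die, which destroys the owning actor.
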(event EventBeginPlay
  (Variables|Default|SetHealth (Variables|Default|GetMaxHealth)))

(event EventTick
  (params (DeltaSeconds :type Float%20%28single-precision%29)))

(fn ReceiveDamage
  (params (Damage :type Float%20%28double-precision%29))
  (if (<= (- (Variables|Default|GetHealth) Damage) 0.0)
    (Variables|Default|SetHealth 0.0)
    (CallFunction|Die)
    (else
      (bind _output_get (Variables|Default|SetHealth (- (Variables|Default|GetHealth) Damage)))
      (Development|PrintString (Utilities|String|ToString(Float) _output_get)))))

(fn Die
  (if (<= (Variables|Default|GetHealth) 0.0)
    (Actor|DestroyActor (Components|GetOwner))))