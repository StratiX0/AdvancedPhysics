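; Hovering mine that explodes three seconds after spawning or when its mesh registers a hit.
; Each tick it traces down along the Reference component's up axis and applies a spring-damper force to the mesh, using ground compression and its rate of change.
; Exploding fires the RadialForce impulse, applies full radial damage within that component's radius and destroys the actor.
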(event OnComponentHit(MineMesh)
  (params (HitComponent :type Primitive%20Component%20Object%20Reference) (OtherActor :type Actor%20Object%20Reference) (OtherComp :type Primitive%20Component%20Object%20Reference) (NormalImpulse :type Vector :default "0, 0, 0") (Hit :type Hit%20Result%20Structure%20%28by%20ref%29))
  (CallFunction|Explode))

(event Custom|Explode
  (Class|RadialForceComponent|FireImpulse (Variables|Default|GetRadialForce))
  (Game|Damage|ApplyRadialDamage (Variables|Default|GetDamage) (Transformation|GetWorldLocation (Variables|Default|GetMineMesh)) (Variables|/Script/Engine.RadialForceComponent|GetRadius (Variables|Default|GetRadialForce)) "/Script/Engine.DamageType" 0 (Components|GetOwner) (Game|GetInstigatorController) true "ECC_Visibility")
  (Actor|DestroyActor))

(event EventBeginPlay
  (Utilities|FlowControl|Delay 3.0)
  (CallFunction|Explode))

(event EventTick
  (params (DeltaSeconds :type Float%20%28single-precision%29))
  (bind _minemesh (Variables|Default|GetMineMesh))
  (bind _distance_between_hover_to_ground (Variables|Default|GetDistance%20Between%20Hover%20to%20Ground))
  (bind _returnvalue (Transformation|GetWorldLocation _minemesh))
  (bind (_outhit _returnvalue_2) (Collision|LineTraceByChannel _returnvalue (- _returnvalue (* (Math|Vector|GetUpVector (Variables|Default|GetReference)) (Variables|Default|GetDistance%20Between%20Hover%20to%20Ground))) "TraceTypeQuery1" false 0 (select (Variables|Default|GetDebugLineTrace) "ForOneFrame" "None")))
  (if _returnvalue_2
    (bind _output_get (Variables|Default|SetHoverUpForce (+ (* (/ (- (/ (- _distance_between_hover_to_ground (.Distance (Collision|BreakHitResult _outhit))) _distance_between_hover_to_ground) (Variables|Default|GetPreviousCompression)) (Utilities|Time|GetWorldDeltaSeconds)) (Variables|Default|GetDamping)) (* (/ (- _distance_between_hover_to_ground (.Distance (Collision|BreakHitResult _outhit))) _distance_between_hover_to_ground) (Variables|Default|GetStiffness)))))
    (Variables|Default|SetPreviousCompression (/ (- _distance_between_hover_to_ground (.Distance (Collision|BreakHitResult _outhit))) _distance_between_hover_to_ground))
    (Class|PrimitiveComponent|AddForceatLocation (Variables|Default|GetMineMesh) (* _output_get (Math|Vector|GetUpVector (Variables|Default|GetReference))) (Transformation|GetWorldLocation (Variables|Default|GetMineMesh)) "None")))

(fn ConstructionScript)