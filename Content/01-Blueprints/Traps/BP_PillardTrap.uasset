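; BP_PillardTrap is a pillar trap that endlessly moves its GCPillard component up and down.
; Tick shifts the component's relative Z at a constant, frame-rate-independent speed, flipping the IsTop flag at fixed lower and upper limits to reverse direction.
; When the pillar registers a hit from a BP_Hovercraft, it switches its collision object type to a custom game channel, with no reset afterwards.
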(event OnComponentHit(GC_Pillard)
  (params (HitComponent :type Primitive%20Component%20Object%20Reference) (OtherActor :type Actor%20Object%20Reference) (OtherComp :type Primitive%20Component%20Object%20Reference) (NormalImpulse :type Vector :default "0, 0, 0") (Hit :type Hit%20Result%20Structure%20%28by%20ref%29))
  (Utilities|Casting|CastToBP_Hovercraft OtherActor)
  (Collision|SetCollisionObjectType (Variables|Default|GetGC_Pillard) "ECC_GameTraceChannel1"))

(event EventBeginPlay)

(event Collision|EventActorBeginOverlap
  (params (OtherActor :type Actor%20Object%20Reference)))

(event EventTick
  (params (DeltaSeconds :type Float%20%28single-precision%29))
  (bind _gc_pillard (Variables|Default|GetGC_Pillard))
  (bind _gc_pillard_2 (Variables|Default|GetGC_Pillard))
  (bind _relativelocation (Variables|/Script/Engine.SceneComponent|GetRelativeLocation _gc_pillard_2))
  (bind _relativelocation_2 (Variables|/Script/Engine.SceneComponent|GetRelativeLocation _gc_pillard))
  (if (Variables|Default|GetIsTop)
    (Transformation|SetRelativeLocation (Variables|Default|GetGC_Pillard) (Math|Vector|MakeVector (.x _relativelocation_2) (.y _relativelocation_2) (- (.z _relativelocation_2) (* DeltaSeconds 5e+02))) false false)
    (if (<= (.z _relativelocation_2) -1e+03)
      (Variables|Default|SetIsTop false))
    (else
      (Transformation|SetRelativeLocation (Variables|Default|GetGC_Pillard) (Math|Vector|MakeVector (.x _relativelocation) (.y _relativelocation) (+ (.z _relativelocation) (* DeltaSeconds 5e+02))) false false)
      (if (>= (.z _relativelocation) -1e+02)
        (Variables|Default|SetIsTop true)))))

(fn ConstructionScript)