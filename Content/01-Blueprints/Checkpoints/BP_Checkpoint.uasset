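; BP_Checkpoint is a one-shot trigger that marks a start or finish point for the hovercraft.
; On BeginPlay it caches the GM_Test game mode.
; When a BP_Hovercraft first overlaps its Box, it sets IsPassed and calls the start or finish event according to its Type enum.
; Other actors and repeat overlaps are ignored, and any other Type value only marks it passed.
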(event OnComponentBeginOverlap(Box)
  (params (OverlappedComponent :type Primitive%20Component%20Object%20Reference) (OtherActor :type Actor%20Object%20Reference) (OtherComp :type Primitive%20Component%20Object%20Reference) (OtherBodyIndex :type Integer) (bFromSweep :type Boolean) (SweepResult :type Hit%20Result%20Structure%20%28by%20ref%29))
  (Utilities|Casting|CastToBP_Hovercraft OtherActor)
  (if (not (Variables|Default|GetIsPassed))
    (Variables|Default|SetIsPassed true)
    (if (Utilities|Enum|Equal(Enum) (Variables|Default|GetType) "NewEnumerator1")
      (Default|CallFinishEvent)
      (elif (Utilities|Enum|Equal(Enum) (Variables|Default|GetType) "NewEnumerator0")
        (Default|CallStartEvent)))))

(event EventBeginPlay
  (bind _asgm_test (Utilities|Casting|CastToGM_Test (Game|GetGameMode)))
  (Variables|Default|SetGameMode _asgm_test))

(event Collision|EventActorBeginOverlap
  (params (OtherActor :type Actor%20Object%20Reference)))

(event EventTick
  (params (DeltaSeconds :type Float%20%28single-precision%29)))

(fn ConstructionScript)